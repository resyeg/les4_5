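; BP_DestructScaleCube is an actor Blueprint that shrinks a little each time another actor begins overlapping it.
; Each overlap reduces the scale stored in ActorsTransform by a fixed uniform step, applies it to the actor, saves it back and prints the value.
; No lower limit or destroy call stops the shrinking.
; BeginPlay and Tick are disabled, and the construction script only calls its parent.
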(event EventBeginPlay
  (|CallParentFunction) ; This node is disabled and will not be called.\nDrag off pins to build functionality.
)

(event Collision|EventActorBeginOverlap
  (params (OtherActor :type Actor%20Object%20Reference))
  (|CallParentFunction OtherActor)
  (Transformation|SetActorScale3D (- (.scale (Variables|Default|GetActorsTransform)) "0.050000,0.050000,0.050000"))
  (Variables|Default|SetActorsTransform (Math|Transform|MakeTransform "0, 0, 0" "0, 0, 0" (- (.scale (Variables|Default|GetActorsTransform)) "0.050000,0.050000,0.050000")))
  (Development|PrintString (Utilities|String|ToString(Vector) (- (.scale (Variables|Default|GetActorsTransform)) "0.050000,0.050000,0.050000"))))

(event EventTick
  (params (DeltaSeconds :type Float%20%28single-precision%29))
  (|CallParentFunction DeltaSeconds) ; This node is disabled and will not be called.\nDrag off pins to build functionality.
)

(fn ConstructionScript
  (|CallParentFunction))