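; BP_Ball is a ball actor that moves in a straight line and bounces off whatever blocks it.
; Each Tick it does a swept world offset along Direction at Speed, scaled by delta time.
; A blocking hit reflects Direction through GetReflectionVector using the X and Y of the hit normal.
; Each bounce also lowers Speed by a fixed fraction of its starting value, computed on BeginPlay, until it reaches MinSpeed.
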(event EventBeginPlay
  (Variables|Default|SetDeltaSpeed (* (Variables|Default|GetSpeed) 0.1)))

(event Collision|EventActorBeginOverlap
  (params (OtherActor :type Actor%20Object%20Reference)))

(event EventTick
  (params (DeltaSeconds :type Float%20%28single-precision%29))
  (bind _minspeed (Variables|Default|GetMinSpeed))
  (bind _sweephitresult (Transformation|AddActorWorldOffset (* (* (Variables|Default|GetDirection) (Variables|Default|GetSpeed)) DeltaSeconds) true))
  (if (.bBlockingHit (Collision|BreakHitResult _sweephitresult))
    (Variables|Default|SetDirection (Math|Vector|GetReflectionVector (Variables|Default|GetDirection) (Math|Vector|MakeVector (.x (.Normal (Collision|BreakHitResult _sweephitresult))) (.y (.Normal (Collision|BreakHitResult _sweephitresult))) 0.0)))
    (if (> (Variables|Default|GetSpeed) _minspeed)
      (Variables|Default|SetSpeed (- (Variables|Default|GetSpeed) (Variables|Default|GetDeltaSpeed)))
      (if (> _minspeed (Variables|Default|GetSpeed))
        (Variables|Default|SetSpeed _minspeed)))))

(fn ConstructionScript)